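; A password-locked safe ("cofre") that holds a key for the player.
; UseItem shows a password widget until the Senha flag is set; afterwards it shares a DoOnce with the senhacorreta event.
; A FlipFlop first swings the door open by timeline and outlines the keys via custom depth, resetting the DoOnce when finished.
; The next trigger hides the keys and sets Chave on the FirstPersonCharacter.
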(event Custom|senhacorreta
  (bind _keys_keyholder (Variables|Default|Getkeys_keyholder))
  (Utilities|FlowControl|DoOnce false :!label _label
    (:Completed
      (Collision|SetCollisionEnabled (Variables|Default|Getuntitled) "NoCollision")
      (Utilities|FlowControl|FlipFlop
        (:A
          (for _array_element (Components|GetChildrenComponents _keys_keyholder false)
            (bind _asprimitive_component (Utilities|Casting|CastToPrimitiveComponent _array_element))
            (Rendering|SetRenderCustomDepth _asprimitive_component true))
          (bind _newtrack_0 (Timeline|Timeline_0 PlayFromStart)
            (:Update
              (Transformation|SetRelativeRotation (Variables|Default|Getuntitled) (Math|Rotator|MakeRotator 0.0 0.0 (Math|Float|Lerp -5.401374 -1.2e+02 _newtrack_0)) false false))
            (:Finished
              (Collision|SetCollisionEnabled (Variables|Default|Getuntitled) "QueryAndPhysics")
              (goto _label Reset))))
        (:B
          (Rendering|SetVisibility _keys_keyholder false true)
          (bind _asfirst_person_character (Utilities|Casting|CastToFirstPersonCharacter (Game|GetPlayerCharacter 0)))
          (Variables|/Game/StarterContent/FirstPersonBP/Blueprints/FirstPersonCharacter.FirstPersonCharacter_C|Setchave _asfirst_person_character true))))))

(event EventBeginPlay)

(event Collision|EventActorBeginOverlap
  (params (OtherActor :type Actor%20Object%20Reference)))

(event EventTick
  (params (DeltaSeconds :type Float%20%28single-precision%29)))

(event EventUseItem
  (bind _keys_keyholder (Variables|Default|Getkeys_keyholder))
  (if (Variables|Default|Getsenha)
    (Utilities|FlowControl|DoOnce false :!label _label
      (:Completed
        (Collision|SetCollisionEnabled (Variables|Default|Getuntitled) "NoCollision")
        (Utilities|FlowControl|FlipFlop
          (:A
            (for _array_element (Components|GetChildrenComponents _keys_keyholder false)
              (bind _asprimitive_component (Utilities|Casting|CastToPrimitiveComponent _array_element))
              (Rendering|SetRenderCustomDepth _asprimitive_component true))
            (bind _newtrack_0 (Timeline|Timeline_0 PlayFromStart)
              (:Update
                (Transformation|SetRelativeRotation (Variables|Default|Getuntitled) (Math|Rotator|MakeRotator 0.0 0.0 (Math|Float|Lerp -5.401374 -1.2e+02 _newtrack_0)) false false))
              (:Finished
                (Collision|SetCollisionEnabled (Variables|Default|Getuntitled) "QueryAndPhysics")
                (goto _label Reset))))
          (:B
            (Rendering|SetVisibility _keys_keyholder false true)
            (bind _asfirst_person_character (Utilities|Casting|CastToFirstPersonCharacter (Game|GetPlayerCharacter 0)))
            (Variables|/Game/StarterContent/FirstPersonBP/Blueprints/FirstPersonCharacter.FirstPersonCharacter_C|Setchave _asfirst_person_character true)))))
    (else
      (bind _returnvalue (UserInterface|CreateWidget "/Game/widget/senha.senha_C" (Game|GetPlayerController 0)))
      (UserInterface|Viewport|AddtoViewport _returnvalue 0))))

(fn ConstructionScript)