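; Interactable small table (Mesinha) with a sliding drawer holding a battery (Pilha) that enables the player's flashlight.
; UseItem toggles the drawer open or closed with a Timeline-driven lerp, gated by a DoOnce that resets when the movement finishes.
; Opening highlights the battery through custom depth until it is collected.
; Using the open drawer collects it, setting Lanterna on FirstPersonCharacter and hiding the battery as the drawer closes.
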(event EventBeginPlay)

(event Collision|EventActorBeginOverlap
  (params (OtherActor :type Actor%20Object%20Reference)))

(event EventTick
  (params (DeltaSeconds :type Float%20%28single-precision%29)))

(event EventUseItem
  (Utilities|FlowControl|DoOnce false :!label _label
    (:Completed
      (if (or (Variables|Default|Getpilhaon) (not (Variables|Default|Getaberta)))
        (if (Variables|Default|Getpilhaon)
          _
          (else
            (Rendering|SetRenderCustomDepth (Variables|Default|Getpilha) true)))
        (else
          (Variables|Default|Setpilhaon true)
          (bind _asfirst_person_character (Utilities|Casting|CastToFirstPersonCharacter (Game|GetPlayerCharacter 0)))
          (Variables|/Game/StarterContent/FirstPersonBP/Blueprints/FirstPersonCharacter.FirstPersonCharacter_C|Setlanterna _asfirst_person_character true)
          (Rendering|SetVisibility (Variables|Default|Getpilha) false false)))
      (if (Variables|Default|Getaberta)
        (Variables|Default|Setaberta false)
        (bind _abre_fecha (Timeline|Timeline_0 ReverseFromEnd)
          (:Update
            (Transformation|SetRelativeLocation (Variables|Default|GetIKEA_Alex_Cube_010) (Math|Vector|MakeVector (Math|Float|Lerp 0.0 3e+01 _abre_fecha) 0.0 0.0) false false))
          (:Finished
            (goto _label Reset)))
        (else
          (Variables|Default|Setaberta true)
          (Timeline|Timeline_0 PlayFromStart))))))

(fn ConstructionScript)