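; Key-locked door that serves as an end trigger, responding to UseItem based on the player's Chave (key) flag.
; With the key, it runs once: shows the Fim widget, disables player input and swings the door leaf open by timeline, with collision off while moving.
; Without it, it shows Fim flagged Incorreta for a few seconds, with a DoOnce preventing stacked messages.
; The FlipFlop's closing branch is unreachable because the first DoOnce never resets.
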(event EventBeginPlay)

(event Collision|EventActorBeginOverlap
  (params (OtherActor :type Actor%20Object%20Reference)))

(event EventTick
  (params (DeltaSeconds :type Float%20%28single-precision%29)))

(event EventUseItem
  (bind _asfirst_person_character (Utilities|Casting|CastToFirstPersonCharacter (Game|GetPlayerCharacter 0)))
  (if (Variables|/Game/StarterContent/FirstPersonBP/Blueprints/FirstPersonCharacter.FirstPersonCharacter_C|Getchave _asfirst_person_character)
    (Utilities|FlowControl|DoOnce false
      (:Completed
        (bind _returnvalue (UserInterface|CreateWidget "/Game/widget/fim.fim_C"))
        (Variables|/Game/widget/fim.fim_C|Setincorreta _returnvalue false)
        (UserInterface|Viewport|AddtoViewport _returnvalue 0)
        (Input|DisableInput (Game|GetPlayerCharacter 0) 0)
        (Collision|SetCollisionEnabled (Variables|Default|GetParametricDoor-V1__doorLeaf) "NoCollision")
        (Utilities|FlowControl|FlipFlop
          (:A
            (bind _newtrack_0 (Timeline|Timeline_0 PlayFromStart)
              (:Update
                (Transformation|SetRelativeRotation (Variables|Default|GetParametricDoor-V1__doorLeaf) (Math|Rotator|MakeRotator 0.0 0.0 (Math|Float|Lerp 0.0 -1.1e+02 _newtrack_0)) false false))
              (:Finished
                (Collision|SetCollisionEnabled (Variables|Default|GetParametricDoor-V1__doorLeaf) "QueryAndPhysics"))))
          (:B
            (Timeline|Timeline_0 ReverseFromEnd)))))
    (else
      (Utilities|FlowControl|DoOnce false :!label _label
        (:Completed
          (bind _returnvalue_2 (UserInterface|CreateWidget "/Game/widget/fim.fim_C"))
          (Variables|/Game/widget/fim.fim_C|Setincorreta _returnvalue_2 true)
          (UserInterface|Viewport|AddtoViewport _returnvalue_2 0)
          (Utilities|FlowControl|Delay 3.0)
          (Widget|RemovefromParent _returnvalue_2)
          (goto _label Reset))))))

(fn ConstructionScript)